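; Init Blueprint that syncs four-light controls and their timed schedules between the GI_Init widget and a Firebase database under "carte2".
; On BeginPlay it reads slash-delimited light states, intensities and schedule entries into the widget, and resets etatHoraire to 0.
; It binds GM_Aqua event dispatchers to write light changes, schedule additions, deletions and activation back to Firebase.
; The clock-reading timer is never wired to run.
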(event `getHeure`
  ;[1 1 1] heures
  (bind _output_get (set `self.heure` (`KismetMathLibrary.GetHour` (`KismetMathLibrary.Now`))))
  (bind _output_get_2 (set `self.minutes` (`KismetMathLibrary.GetMinute` (`KismetMathLibrary.Now`)))))

(event `lumiereSelect`
  ;[1 1 1] send gui lumiere selectionnee
  (bind _foundwidgets (`WidgetBlueprintLibrary.GetAllWidgetsOfClass` "/Game/Map/GI_Init.GI_Init_C"))
  (`/Game/Map/GI_Init.InitGuiVariable` (`|GetArrayItem` _foundwidgets) (`self.lumiereEtatL1`) (`self.lumiereEtatL2`) (`self.lumiereEtatL3`) (`self.lumiereEtatL4`) (`self.intensiteL1`) (`self.intensiteL2`) (`self.intensiteL3`) (`self.intensiteL4`)))

(event `self.ReceiveBeginPlay`
  ;[1 1 1] initaialisation et recuperation taille de la taille liste horaire
  (bind _asgm_aqua (cast `/Game/Map/GM_Aqua` (`GameplayStatics.GetGameMode`)))
  (set `self.As GM Aqua` _asgm_aqua)
  (set `self.Reference` (`Database.GetReference` (`Database.GetInstance`)))
  (bind (_error _snapshot) (`DatabaseQueryGetValue.GetValue` (`DatabaseReference.Child` (`self.Reference`) "carte2/horlogeLengt"))
    (:`OnDataReceived`
      (set `self.horlogeLengtArray` (`VariantLibrary.ToString` (`DataSnapshot.GetValue` _snapshot)))
      (`|ExecutionSequence`
        (:`then_0`
          ;[1 1 1] recuperation info lumiere base de donnee
          (bind (_error_2 _snapshot_2) (`DatabaseQueryGetValue.GetValue` (`DatabaseReference.Child` (`self.Reference`) "carte2/lumiere"))
            (:`OnDataReceived`
              (bind _returnvalue (`DataSnapshot.GetValue` _snapshot_2))
              (`KismetSystemLibrary.PrintString` (`VariantLibrary.ToString` _returnvalue) false false (struct :`R` 1.0 :`B` 0.068094 :`A` 1.0) 10.0)
              (bind _returnvalue_2 (`KismetStringLibrary.ParseIntoArray` (`VariantLibrary.ToString` _returnvalue) "/"))
              (set `self.HorlogeEtat` (`KismetStringLibrary.Conv_StringToInt` (`|GetArrayItem` _returnvalue_2)))
              (set `self.lumiereEtatL1` (`KismetStringLibrary.Conv_StringToInt` (`|GetArrayItem` _returnvalue_2 1)))
              (set `self.lumiereEtatL2` (`KismetStringLibrary.Conv_StringToInt` (`|GetArrayItem` _returnvalue_2 2)))
              (set `self.lumiereEtatL3` (`KismetStringLibrary.Conv_StringToInt` (`|GetArrayItem` _returnvalue_2 3)))
              (set `self.lumiereEtatL4` (`KismetStringLibrary.Conv_StringToInt` (`|GetArrayItem` _returnvalue_2 4)))
              (set `self.intensiteL1` (`KismetStringLibrary.Conv_StringToInt` (`|GetArrayItem` _returnvalue_2 5)))
              (set `self.intensiteL2` (`KismetStringLibrary.Conv_StringToInt` (`|GetArrayItem` _returnvalue_2 6)))
              (set `self.intensiteL3` (`KismetStringLibrary.Conv_StringToInt` (`|GetArrayItem` _returnvalue_2 7)))
              (set `self.intensiteL4` (`KismetStringLibrary.Conv_StringToInt` (`|GetArrayItem` _returnvalue_2 8)))
              (`self.lumiereselect`)
              ;[1 1 1] send param lumiere firebase
              (add `/Game/Map/GM_Aqua.EDLumiereParam` (`self.As GM Aqua`) (delegate `LumiereParam`)))))
        (:`then_1`
          ;[1 1 1] ecriture dictonnaire horloge et envois sur la base de donnée
          (add `/Game/Map/GM_Aqua.EDLumiereHorloge` (`self.As GM Aqua`) (delegate `EventLumiereHorloge`)))
        (:`then_3`
          ;[1 1 1] supp id horloge  sur la base de donnée
          (add `/Game/Map/GM_Aqua.EDLumiereHorlogeSupp` (`self.As GM Aqua`) (delegate `idsupp`)))
        (:`then_4`
          ;[1 1 1] recuperation horaire lumiere base de donnee + mise a jour liste hud horloge
          (for _index (range 1 (+ (`KismetStringLibrary.Conv_StringToInt` (`self.horlogeLengtArray`)) 1))
            (bind _returnvalue_3 (`KismetStringLibrary.Conv_IntToString` _index))
            (`KismetSystemLibrary.PrintString` _returnvalue_3 false false (struct :`R` 1.0 :`B` 0.068094 :`A` 1.0) 10.0)
            (bind (_error_3 _snapshot_3) (`DatabaseQueryGetValue.GetValue` (`DatabaseReference.Child` (`self.Reference`) (`KismetStringLibrary.Concat_StrStr` "carte2/lumiereHorloge/" _returnvalue_3)))
              (:`OnDataReceived`
                (bind _foundwidgets (`WidgetBlueprintLibrary.GetAllWidgetsOfClass` "/Game/Map/GI_Init.GI_Init_C"))
                (bind _returnvalue_4 (`KismetStringLibrary.ParseIntoArray` (`VariantLibrary.ToString` (`DataSnapshot.GetValue` _snapshot_3)) "/"))
                (`/Game/Map/GI_Init.Add Liste Horaire` (`|GetArrayItem` _foundwidgets) (`|GetArrayItem` _returnvalue_4) (`|GetArrayItem` _returnvalue_4 1) (`|GetArrayItem` _returnvalue_4 2) (`|GetArrayItem` _returnvalue_4 3) (`|GetArrayItem` _returnvalue_4 4) (`|GetArrayItem` _returnvalue_4 5) (`|GetArrayItem` _returnvalue_4 6) (`|GetArrayItem` _returnvalue_4 7) (`|GetArrayItem` _returnvalue_4 8) (`|GetArrayItem` _returnvalue_4 9))))))
        (:`then_5`
          ;[1 1 1] mise a jour etat de l horloge sur base de donnée
          (add `/Game/Map/GM_Aqua.EDLumiereHorlogeActive` (`self.As GM Aqua`) (delegate `CustomEvent_0`)))
        (:`then_6`
          (`SetValueProxy.SetValue` (`DatabaseReference.Child` (`self.Reference`) "carte2/etatHoraire/") (`VariantLibrary.FromString` (`KismetStringLibrary.Conv_IntToString` 0))))))))

(event `LumiereParam`
  (params (e1 :type Integer) (e2 :type Integer) (e3 :type Integer) (e4 :type Integer) (i1 :type Integer) (i2 :type Integer) (i3 :type Integer) (i4 :type Integer))
  ;[1 1 1] send param lumiere firebase
  (`SetValueProxy.SetValue` (`DatabaseReference.Child` (`self.Reference`) "carte2/lumiere") (`VariantLibrary.FromString` (`KismetStringLibrary.Concat_StrStr` (`KismetStringLibrary.Conv_IntToString` (`self.HorlogeEtat`)) "/" (`KismetStringLibrary.Conv_IntToString` e1) "/" (`KismetStringLibrary.Conv_IntToString` e2) "/" (`KismetStringLibrary.Conv_IntToString` e3) "/" (`KismetStringLibrary.Conv_IntToString` e4) "/" (`KismetStringLibrary.Conv_IntToString` i1) "/" (`KismetStringLibrary.Conv_IntToString` i2) "/" (`KismetStringLibrary.Conv_IntToString` i3) "/" (`KismetStringLibrary.Conv_IntToString` i4)))))

(event `CustomEvent_0`
  (params (valeurHorlogeActive :type Integer))
  ;[1 1 1] mise a jour etat de l horloge sur base de donnée
  (`SetValueProxy.SetValue` (`DatabaseReference.Child` (`self.Reference`) "carte2/etatHoraire/") (`VariantLibrary.FromString` (`KismetStringLibrary.Conv_IntToString` valeurHorlogeActive))))

(event `EventLumiereHorloge`
  (params (id :type Integer))
  ;[1 1 1] ecriture dictonnaire horloge et envois sur la base de donnée
  (`KismetSystemLibrary.PrintString` "Hello" false)
  (`SetValueProxy.SetValue` (`DatabaseReference.Child` (`self.Reference`) "carte2/horlogeLengt/") (`VariantLibrary.FromString` (`KismetStringLibrary.Conv_IntToString` id))
    (:`OnSet`
      (bind _foundwidgets (`WidgetBlueprintLibrary.GetAllWidgetsOfClass` "/Game/Map/GI_Init.GI_Init_C"))
      (`SetValueProxy.SetValue` (`DatabaseReference.Child` (`DatabaseReference.Child` (`self.Reference`) "carte2/lumiereHorloge/") (`KismetStringLibrary.Conv_IntToString` id)) (`VariantLibrary.FromString` (`BlueprintMapLibrary.Map_Find` (`/Game/Map/GI_Init.TableauHoraireTime` (`|GetArrayItem` _foundwidgets)) id))))))

(event `idsupp`
  (params (id :type Integer))
  ;[1 1 1] supp id horloge  sur la base de donnée
  (`KismetSystemLibrary.PrintString` (`KismetStringLibrary.Conv_IntToString` id) false false)
  (`SetValueProxy.SetValue` (`DatabaseReference.Child` (`self.Reference`) "carte2/horlogeLengt/") (`VariantLibrary.FromString` (`KismetStringLibrary.Conv_IntToString` id))
    (:`OnSet`
      (`RemoveValueProxy.RemoveValue` (`DatabaseReference.Child` (`DatabaseReference.Child` (`self.Reference`) "carte2/lumiereHorloge/") (`KismetStringLibrary.Conv_IntToString` (+ id 1)))))))

(fn `UserConstructionScript`)